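; Cube House "S" room: an inspectable multi-floor building with case objects revealed in three stages.
; Timeline events fade walls via a dynamic material, open windows, move the floor elevator, and cycle separation and floor splitting, with state checks coordinating them.
; Time-change events toggle visibility and interactivity while sliding the actor.
; Case events unhide clue boxes and enable their collision; SetRelatedObjects links boxes to CubeHouseM and LightHouseM counterparts through GI_Room_Instance.
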(event Custom|HideWalls
  ;[1 1 1] HideWalls
  (bind _isa (Utilities|FlowControl|FlipFlop)
    (:A
      (bind _fade (Timeline|WallsFade Play)
        (:Update
          (Rendering|Material|SetScalarParameterValue (Variables|组件|GetDynamicConcreteMat) "FadeAmount" _fade :!class /Script/Engine.MaterialInstanceDynamic))
        (:Finished
          (Variables|Default|SetisWallsHide _isa))))
    (:B
      (Timeline|WallsFade Reverse))))

(event Custom|ThirdCaseStart
  (bind _roominstanceref (Variables|Reference|GetRoomInstanceRef))
  (bind _3rdcasebox (Variables|Default|Get3rdCaseBox))
  (Utilities|FlowControl|Delay 1.0)
  (CallFunction|OpenWindows)
  (Utilities|FlowControl|Delay 1.0)
  (for _array_element (Components|GetChildrenComponents _3rdcasebox false)
    (Development|SetHiddeninGame _array_element false true)
    (bind _asbp_interactive_basic (Utilities|Casting|CastToBP_Interactive_Basic (Variables|/Script/Engine.ChildActorComponent|GetChildActor _3rdcasebox)))
    (Default|SetRelatedCollision _asbp_interactive_basic "QueryOnly")
    (Utilities|Array|Add (Variables|Default|GetInteractiveBoxes) _3rdcasebox)
    (Development|ExecuteConsoleCommand "ce SplitFloors" 0)
    (Utilities|FlowControl|Delay 0.5)
    (Default|ClearClickedObjects _roominstanceref)
    (Default|CustomClickEvent _asbp_interactive_basic)
    (Default|UpdateClickedObject _roominstanceref _asbp_interactive_basic)))

(event Custom|FirstCaseStart
  (bind _1stcasebox (Variables|Default|Get1stCaseBox))
  (for _array_element (Components|GetChildrenComponents _1stcasebox false)
    (Development|SetHiddeninGame _array_element false true)
    (bind _asbp_interactive_basic (Utilities|Casting|CastToBP_Interactive_Basic (Variables|/Script/Engine.ChildActorComponent|GetChildActor _1stcasebox)))
    (Default|SetRelatedCollision _asbp_interactive_basic "QueryOnly")
    (Utilities|Array|Add (Variables|Default|GetInteractiveBoxes) _1stcasebox)))

(event Custom|SecondCaseStart
  (bind _sm_cordwrap_01a3 (Variables|Default|GetSM_CordWrap_01a3))
  (bind _2ndcasebox (Variables|Default|Get2ndCaseBox))
  (Transformation|AttachComponentToComponent _sm_cordwrap_01a3 (Variables|Default|GetSM_CordWrap_01a1) "None" "KeepWorld" "KeepWorld" "KeepWorld" false)
  (Transformation|SetRelativeLocation _sm_cordwrap_01a3 (Math|Vector|MakeVector 0.0 0.0 1e+01) false false)
  (Transformation|SetRelativeRotation _sm_cordwrap_01a3 (Math|Rotator|MakeRotator 0.0 0.0 0.0) false false)
  (for _array_element (Components|GetChildrenComponents _2ndcasebox false)
    (Development|SetHiddeninGame _array_element false true)
    (bind _asbp_interactive_basic (Utilities|Casting|CastToBP_Interactive_Basic (Variables|/Script/Engine.ChildActorComponent|GetChildActor _2ndcasebox)))
    (Default|SetRelatedCollision _asbp_interactive_basic "QueryOnly")
    (Utilities|Array|Add (Variables|Default|GetInteractiveBoxes) _2ndcasebox)))

(event Custom|OpenWindows
  (bind _sm_picture_2 (Variables|Props|GetSM_Picture_2))
  ;[1 1 1] OpenWindows
  (Utilities|FlowControl|Sequence
    (:then_0
      (Utilities|FlowControl|FlipFlop
        (:A
          (bind _angle (Timeline|WindowOpen1 Play)
            (:Update
              (Transformation|SetRelativeRotation (Variables|Default|GetWindowContainer) (Math|Rotator|MakeRotator _angle 0.0 0.0) false false))))
        (:B
          (Timeline|WindowOpen1 Reverse))))
    (:then_1
      (Utilities|FlowControl|DoOnce false
        (:Completed
          (bind _output_get (Variables|Default|SetpictureTransformTemp (Transformation|GetRelativeTransform _sm_picture_2)))
          (bind (_direction _x _y _z _anglex _angley _anglez) (Timeline|WindowOpen2 Play)
            (:Update
              (Transformation|SetRelativeTransform _sm_picture_2 (Math|Transform|MakeTransform (+ (.location _output_get) (Math|Vector|RotateVector (* (Math|Vector|MakeVector _x _y _z) (.scale _output_get)) (.rotation _output_get))) (Math|Rotator|MakeRotator (+ _anglex (.Roll (Math|Rotator|BreakRotator (.rotation _output_get)))) (+ _angley (.Pitch (Math|Rotator|BreakRotator (.rotation _output_get)))) (+ _anglez (.Yaw (Math|Rotator|BreakRotator (.rotation _output_get))))) (.scale _output_get)) false false))))))))

(event EventBeginPlay
  (Utilities|FlowControl|Sequence
    (:then_0
      (bind _asgi_room_instance (Utilities|Casting|CastToGI_Room_Instance (Game|GetGameInstance)))
      (Variables|Reference|SetRoomInstanceRef _asgi_room_instance))
    (:then_1
      (bind _returnvalue (Rendering|Material|CreateDynamicMaterialInstance "/Game/WorldInferRules/Materials/M_Exterior_Concrete.M_Exterior_Concrete" "None" "None" :!class /Script/Engine.KismetMaterialLibrary))
      (bind _output_get (Variables|组件|SetDynamicConcreteMat _returnvalue))
      (for _array_element (Variables|组件|GetWalls)
        (Rendering|Material|SetMaterial _array_element 1 _output_get)
        (Rendering|Material|SetMaterial (Variables|Default|Get回形馆_0Floor) 0 _output_get)))))

(event EventSeparateHouse
  (bind _sepcontainer (Variables|ContainerComps|GetSepContainer))
  (bind _relativelocation (Variables|/Script/Engine.SceneComponent|GetRelativeLocation _sepcontainer))
  ;[1 1 1] SeparateHouse
  (if (!= (Variables|Default|GetSplitState) 1)
    (Utilities|FlowControl|MultiGate false true -1
      (:Out%200
        (Variables|State|SetSeparateState 0)
        (bind _angle (Timeline|HouseSeparate1 Play)
          (:Update
            (Transformation|SetRelativeRotation (Variables|ContainerComps|GetSepContainer) (Math|Rotator|MakeRotator 0.0 0.0 _angle) false false))))
      (:Out%201
        (Variables|State|SetSeparateState 1)
        (bind _distance (Timeline|HouseSeparate2 Play)
          (:Update
            (Transformation|SetRelativeLocation _sepcontainer (Math|Vector|MakeVector _distance (.y _relativelocation) (.z _relativelocation)) false false))))
      (:Out%202
        (Variables|State|SetSeparateState 2)
        (Utilities|FlowControl|Sequence
          (:then_0
            (Timeline|HouseSeparate1 Reverse))
          (:then_1
            (Timeline|HouseSeparate2 Reverse)))))))

(event EventChangeTimeSp
  (bind _self self)
  (bind _defaultsceneroot (Variables|组件|GetDefaultSceneRoot))
  (bind _returnvalue (Transformation|GetWorldLocation _defaultsceneroot))
  (bind _bhidden (Variables|Default|GetbHidden _self))
  (bind _returnvalue_2 (not _bhidden))
  ;[1 1 1] ChangeTime
  (Rendering|SetActorHiddenInGame _returnvalue_2)
  (CallFunction|MovetoHide _bhidden)
  (CallFunction|EnableInteractive _returnvalue_2)
  (bind _move (Timeline|TimeChange1 PlayFromStart)
    (:Update
      (Transformation|SetWorldLocation _defaultsceneroot (Math|Vector|MakeVector (.x _returnvalue) _move (.z _returnvalue)) false false))))

(event EventChangeTimeNormal
  (bind _self self)
  (bind _defaultsceneroot (Variables|组件|GetDefaultSceneRoot))
  (bind _returnvalue (Transformation|GetWorldLocation _defaultsceneroot))
  (bind _bhidden (Variables|Default|GetbHidden _self))
  (bind _returnvalue_2 (not _bhidden))
  ;[1 1 1] ChangeTime
  (Rendering|SetActorHiddenInGame _returnvalue_2)
  (CallFunction|MovetoHide _bhidden)
  (CallFunction|EnableInteractive _returnvalue_2)
  (bind _move (Timeline|TimeChange2 ReverseFromEnd)
    (:Update
      (Transformation|SetWorldLocation _defaultsceneroot (Math|Vector|MakeVector (.x _returnvalue) _move (.z _returnvalue)) false false))))

(event EventSplitFloors
  (bind _sepcontainer (Variables|ContainerComps|GetSepContainer))
  (bind _relativelocation (Variables|/Script/Engine.SceneComponent|GetRelativeLocation _sepcontainer))
  ;[1 1 1] SplitFloors
  (if (not (Variables|状态|GetisElevatorMoving))
    (Utilities|WhileLoopwithDelay (> (Variables|状态|GetElevatorState) 0) 1.0
      (:LoopBody
        (CallFunction|MoveUpFloor))
      (:Completed
        (Utilities|FlowControl|MultiGate false true -1
          (:Out%200
            (Variables|Default|SetSplitState 0)
            (bind (_direction _roof _floor3 _floor2) (Timeline|FloorSplit1 Play)
              (:Update
                (Utilities|SplitFloorbyDistance (Math|Vector|MakeVector (- 0.0 (stale _x)) (- 0.0 (stale _y)) (- _roof (stale _z))) (Math|Vector|MakeVector (stale _x) (- 0.0 (stale _y)) _floor3) (Math|Vector|MakeVector (- 0.0 (stale _x)) (stale _y) (+ _floor2 (stale _z))) (Math|Vector|MakeVector (stale _x) (stale _y) (+ (stale _z) (stale _z))) :!label _label))))
          (:Out%201
            (Variables|Default|SetSplitState 1)
            (Utilities|FlowControl|Sequence
              (:then_0
                ;[1 1 1] SeparateHouse
                (switch int (Variables|State|GetSeparateState)
                  (:0
                    (Utilities|FlowControl|Sequence
                      (:then_0
                        (Utilities|FlowControl|MultiGate false true -1) ; enters at Reset
                      )
                      (:then_1
                        (bind _angle (Timeline|HouseSeparate1 Reverse)
                          (:Update
                            (Transformation|SetRelativeRotation (Variables|ContainerComps|GetSepContainer) (Math|Rotator|MakeRotator 0.0 0.0 _angle) false false))))))
                  (:1
                    (Utilities|FlowControl|Sequence
                      (:then_0
                        (Utilities|FlowControl|MultiGate false true -1) ; enters at Reset
                      )
                      (:then_1
                        (Utilities|FlowControl|Sequence
                          (:then_0
                            (Timeline|HouseSeparate1 Reverse))
                          (:then_1
                            (bind _distance (Timeline|HouseSeparate2 Reverse)
                              (:Update
                                (Transformation|SetRelativeLocation _sepcontainer (Math|Vector|MakeVector _distance (.y _relativelocation) (.z _relativelocation)) false false))))))))))
              (:then_1
                (bind (_direction_2 _x _y _z) (Timeline|FloorSplit2 Play)
                  (:Update
                    (goto _label))))))
          (:Out%202
            (Variables|Default|SetSplitState 2)
            (Utilities|FlowControl|Sequence
              (:then_0
                (Timeline|FloorSplit1 Reverse))
              (:then_1
                (Timeline|FloorSplit2 Reverse)))))))))

(event EventMoveDownFloor
  ;[1 1 1] Elevator
  (if (and (< (Variables|状态|GetElevatorState) 2) (not (Variables|状态|GetisElevatorMoving)))
    (Variables|状态|SetisElevatorMoving true)
    (Math|Integer|IncrementInt (Variables|状态|GetElevatorState)
      (:%20%20
        (Utilities|StoreFloorTempLocation)
        (bind _goup (Timeline|FloorMoveDown PlayFromStart)
          (:Update
            (Utilities|AddFloorDeltaLocation (Math|Vector|MakeVector 0.0 0.0 _goup)))
          (:Finished
            (Variables|状态|SetisElevatorMoving false)))))))

(event EventMoveUpFloor
  ;[1 1 1] Elevator
  (if (and (> (Variables|状态|GetElevatorState) 0) (not (Variables|状态|GetisElevatorMoving)))
    (Variables|状态|SetisElevatorMoving true)
    (Math|Integer|DecrementInt (Variables|状态|GetElevatorState)
      (:%20%20
        (Utilities|StoreFloorTempLocation)
        (bind _goup (Timeline|FloorMoveUp PlayFromStart)
          (:Update
            (Utilities|AddFloorDeltaLocation (Math|Vector|MakeVector 0.0 0.0 _goup)))
          (:Finished
            (Variables|状态|SetisElevatorMoving false)))))))

(fn ConstructionScript
  (Utilities|FlowControl|Sequence
    (:then_0
      (Variables|组件|SetWalls (Utilities|Array|MakeArray (Variables|WallComps|Get回形馆_1FloorWallS) (Variables|WallComps|Get回形馆_2FloorWallS) (Variables|WallComps|Get回形馆_3FloorWallS) (Variables|WallComps|Get回形馆_4RoofWallS) (Variables|WallComps|Get回形馆_3WindowS))))
    (:then_1
      (Variables|Default|SetInteractiveBoxes (Utilities|Array|MakeArray (Variables|BoxComps|GetFloor1Box) (Variables|Default|GetFloor1EBox) (Variables|BoxComps|GetFloor2Box) (Variables|Default|GetFloor2NEBox) (Variables|Default|GetFloor2EBox) (Variables|Default|GetFloor2SEBox) (Variables|BoxComps|GetFloor3Box) (Variables|Default|GetFloor3NEBox) (Variables|Default|GetFloor3EBox) (Variables|Default|GetFloor3SEBox) (Variables|BoxComps|GetFloor4Box))))
    (:then_2
      (Utilities|HideCaseObjectCollision))))

(fn SetRelatedObjects
  (bind _asgi_room_instance (Utilities|Casting|CastToGI_Room_Instance (Game|GetGameInstance)))
  (Utilities|FlowControl|Sequence
    (:then_0
      ;[1 1 1] SetRelatedFloor
      (bind _asbp_interactive_basic (Utilities|Casting|CastToBP_Interactive_Basic (Variables|/Script/Engine.ChildActorComponent|GetChildActor (Variables|/Game/WorldInferRules/BP_Room_CubeHouse_M.BP_Room_CubeHouse_M_C|GetFloor1Box (Variables|/Game/WorldInferRules/GI_Room_Instance.GI_Room_Instance_C|GetcubeHouseM _asgi_room_instance)))))
      (bind _asbp_interactive_basic_2 (Utilities|Casting|CastToBP_Interactive_Basic (Variables|/Script/Engine.ChildActorComponent|GetChildActor (Variables|/Game/WorldInferRules/BP_Room_LightHouse_M.BP_Room_LightHouse_M_C|GetFloor1Box (Variables|/Game/WorldInferRules/GI_Room_Instance.GI_Room_Instance_C|GetlightHouseM _asgi_room_instance)))))
      (bind _asbp_interactive_basic_3 (Utilities|Casting|CastToBP_Interactive_Basic (Variables|/Script/Engine.ChildActorComponent|GetChildActor (Variables|BoxComps|GetFloor1Box))))
      (Variables|/Game/WorldInferRules/BP_Interactive_Basic.BP_Interactive_Basic_C|SetrelatedInteractive _asbp_interactive_basic_3 (Utilities|Array|MakeArray _asbp_interactive_basic))
      (Variables|/Game/WorldInferRules/BP_Interactive_Basic.BP_Interactive_Basic_C|SetrelatedInteractiveSp _asbp_interactive_basic_3 (Utilities|Array|MakeArray _asbp_interactive_basic_2)))
    (:then_1
      (bind _asbp_interactive_basic_4 (Utilities|Casting|CastToBP_Interactive_Basic (Variables|/Script/Engine.ChildActorComponent|GetChildActor (Variables|/Game/WorldInferRules/BP_Room_CubeHouse_M.BP_Room_CubeHouse_M_C|GetFloor2Box (Variables|/Game/WorldInferRules/GI_Room_Instance.GI_Room_Instance_C|GetcubeHouseM _asgi_room_instance)))))
      (bind _asbp_interactive_basic_5 (Utilities|Casting|CastToBP_Interactive_Basic (Variables|/Script/Engine.ChildActorComponent|GetChildActor (Variables|/Game/WorldInferRules/BP_Room_LightHouse_M.BP_Room_LightHouse_M_C|GetFloor2Box (Variables|/Game/WorldInferRules/GI_Room_Instance.GI_Room_Instance_C|GetlightHouseM _asgi_room_instance)))))
      (bind _asbp_interactive_basic_6 (Utilities|Casting|CastToBP_Interactive_Basic (Variables|/Script/Engine.ChildActorComponent|GetChildActor (Variables|BoxComps|GetFloor2Box))))
      (Variables|/Game/WorldInferRules/BP_Interactive_Basic.BP_Interactive_Basic_C|SetrelatedInteractive _asbp_interactive_basic_6 (Utilities|Array|MakeArray _asbp_interactive_basic_4))
      (Variables|/Game/WorldInferRules/BP_Interactive_Basic.BP_Interactive_Basic_C|SetrelatedInteractiveSp _asbp_interactive_basic_6 (Utilities|Array|MakeArray _asbp_interactive_basic_5)))
    (:then_2
      (bind _asbp_interactive_basic_7 (Utilities|Casting|CastToBP_Interactive_Basic (Variables|/Script/Engine.ChildActorComponent|GetChildActor (Variables|/Game/WorldInferRules/BP_Room_CubeHouse_M.BP_Room_CubeHouse_M_C|GetFloor3Box (Variables|/Game/WorldInferRules/GI_Room_Instance.GI_Room_Instance_C|GetcubeHouseM _asgi_room_instance)))))
      (bind _asbp_interactive_basic_8 (Utilities|Casting|CastToBP_Interactive_Basic (Variables|/Script/Engine.ChildActorComponent|GetChildActor (Variables|/Game/WorldInferRules/BP_Room_LightHouse_M.BP_Room_LightHouse_M_C|GetFloor3Box (Variables|/Game/WorldInferRules/GI_Room_Instance.GI_Room_Instance_C|GetlightHouseM _asgi_room_instance)))))
      (bind _asbp_interactive_basic_9 (Utilities|Casting|CastToBP_Interactive_Basic (Variables|/Script/Engine.ChildActorComponent|GetChildActor (Variables|BoxComps|GetFloor3Box))))
      (Variables|/Game/WorldInferRules/BP_Interactive_Basic.BP_Interactive_Basic_C|SetrelatedInteractive _asbp_interactive_basic_9 (Utilities|Array|MakeArray _asbp_interactive_basic_7))
      (Variables|/Game/WorldInferRules/BP_Interactive_Basic.BP_Interactive_Basic_C|SetrelatedInteractiveSp _asbp_interactive_basic_9 (Utilities|Array|MakeArray _asbp_interactive_basic_8)))
    (:then_3
      (bind _asbp_interactive_basic_10 (Utilities|Casting|CastToBP_Interactive_Basic (Variables|/Script/Engine.ChildActorComponent|GetChildActor (Variables|/Game/WorldInferRules/BP_Room_CubeHouse_M.BP_Room_CubeHouse_M_C|GetFloor4Box (Variables|/Game/WorldInferRules/GI_Room_Instance.GI_Room_Instance_C|GetcubeHouseM _asgi_room_instance)))))
      (bind _asbp_interactive_basic_11 (Utilities|Casting|CastToBP_Interactive_Basic (Variables|/Script/Engine.ChildActorComponent|GetChildActor (Variables|/Game/WorldInferRules/BP_Room_LightHouse_M.BP_Room_LightHouse_M_C|GetFloor4Box (Variables|/Game/WorldInferRules/GI_Room_Instance.GI_Room_Instance_C|GetlightHouseM _asgi_room_instance)))))
      (bind _asbp_interactive_basic_12 (Utilities|Casting|CastToBP_Interactive_Basic (Variables|/Script/Engine.ChildActorComponent|GetChildActor (Variables|BoxComps|GetFloor4Box))))
      (Variables|/Game/WorldInferRules/BP_Interactive_Basic.BP_Interactive_Basic_C|SetrelatedInteractive _asbp_interactive_basic_12 (Utilities|Array|MakeArray _asbp_interactive_basic_10))
      (Variables|/Game/WorldInferRules/BP_Interactive_Basic.BP_Interactive_Basic_C|SetrelatedInteractiveSp _asbp_interactive_basic_12 (Utilities|Array|MakeArray _asbp_interactive_basic_11)))
    (:then_4
      ;[1 1 1] SetRelatedRoom
      (bind _asbp_interactive_basic_13 (Utilities|Casting|CastToBP_Interactive_Basic (Variables|/Script/Engine.ChildActorComponent|GetChildActor (Variables|/Game/WorldInferRules/BP_Room_CubeHouse_M.BP_Room_CubeHouse_M_C|GetFloor1EBox (Variables|/Game/WorldInferRules/GI_Room_Instance.GI_Room_Instance_C|GetcubeHouseM _asgi_room_instance)))))
      (bind _asbp_interactive_basic_14 (Utilities|Casting|CastToBP_Interactive_Basic (Variables|/Script/Engine.ChildActorComponent|GetChildActor (Variables|Default|GetFloor1EBox))))
      (Variables|/Game/WorldInferRules/BP_Interactive_Basic.BP_Interactive_Basic_C|SetrelatedInteractive _asbp_interactive_basic_14 (Utilities|Array|MakeArray _asbp_interactive_basic_13)))
    (:then_5
      (bind _asbp_interactive_basic_15 (Utilities|Casting|CastToBP_Interactive_Basic (Variables|/Script/Engine.ChildActorComponent|GetChildActor (Variables|/Game/WorldInferRules/BP_Room_CubeHouse_M.BP_Room_CubeHouse_M_C|GetFloor2EBox (Variables|/Game/WorldInferRules/GI_Room_Instance.GI_Room_Instance_C|GetcubeHouseM _asgi_room_instance)))))
      (bind _asbp_interactive_basic_16 (Utilities|Casting|CastToBP_Interactive_Basic (Variables|/Script/Engine.ChildActorComponent|GetChildActor (Variables|Default|GetFloor2EBox))))
      (Variables|/Game/WorldInferRules/BP_Interactive_Basic.BP_Interactive_Basic_C|SetrelatedInteractive _asbp_interactive_basic_16 (Utilities|Array|MakeArray _asbp_interactive_basic_15)))
    (:then_6
      (bind _asbp_interactive_basic_17 (Utilities|Casting|CastToBP_Interactive_Basic (Variables|/Script/Engine.ChildActorComponent|GetChildActor (Variables|/Game/WorldInferRules/BP_Room_CubeHouse_M.BP_Room_CubeHouse_M_C|GetFloor3EBox (Variables|/Game/WorldInferRules/GI_Room_Instance.GI_Room_Instance_C|GetcubeHouseM _asgi_room_instance)))))
      (bind _asbp_interactive_basic_18 (Utilities|Casting|CastToBP_Interactive_Basic (Variables|/Script/Engine.ChildActorComponent|GetChildActor (Variables|Default|GetFloor3EBox))))
      (Variables|/Game/WorldInferRules/BP_Interactive_Basic.BP_Interactive_Basic_C|SetrelatedInteractive _asbp_interactive_basic_18 (Utilities|Array|MakeArray _asbp_interactive_basic_17)))))