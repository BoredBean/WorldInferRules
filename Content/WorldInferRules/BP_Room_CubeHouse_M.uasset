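; Cube house room actor whose four floor containers shift like an elevator, split apart and link to counterpart rooms.
; Timelines drive elevator moves from stored positions, a dynamic-material wall fade toggle, and a root Y slide for time changes.
; SplitFloors first steps the elevator to state zero, then a looping MultiGate cycles two split stages and a reversal.
; SetRelatedObjects links interactive boxes to CubeHouseS and LightHouseS counterparts through the game instance.
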(event Custom|HideWalls
  ;[1 1 1] HideWalls
  (bind _isa (Utilities|FlowControl|FlipFlop)
    (:A
      (bind _fade (Timeline|WallsFade Play)
        (:Update
          (Rendering|Material|SetScalarParameterValue (Variables|组件|GetDynamicConcreteMat) "FadeAmount" _fade :!class /Script/Engine.MaterialInstanceDynamic))
        (:Finished
          (Variables|Default|SetisWallsHide _isa))))
    (:B
      (Timeline|WallsFade Reverse))))

(event Custom|ThirdCaseStart
  (Utilities|FlowControl|Delay 2.0)
  (Development|SetHiddeninGame (Variables|Default|Get回形馆_0FloorS) false false))

(event EventBeginPlay
  (bind _returnvalue (Rendering|Material|CreateDynamicMaterialInstance "/Game/WorldInferRules/Materials/M_Exterior_Concrete.M_Exterior_Concrete" "None" "None" :!class /Script/Engine.KismetMaterialLibrary))
  (bind _output_get (Variables|组件|SetDynamicConcreteMat _returnvalue))
  (for _array_element (Variables|组件|GetWalls)
    (Rendering|Material|SetMaterial _array_element 1 _output_get)
    (Rendering|Material|SetMaterial (Variables|Default|Get回形馆_0FloorS) 0 _output_get)))

(event EventMoveUpFloor
  ;[1 1 1] Elevator
  (if (and (> (Variables|State|GetElevatorState) 0) (not (Variables|状态|GetisElevatorMoving)))
    (Variables|状态|SetisElevatorMoving true)
    (Math|Integer|DecrementInt (Variables|State|GetElevatorState)
      (:%20%20
        (Utilities|StoreFloorTempLocation)
        (bind _goup (Timeline|FloorMoveUp PlayFromStart)
          (:Update
            (Utilities|AddFloorDeltaLocation (Math|Vector|MakeVector 0.0 0.0 _goup)))
          (:Finished
            (Variables|状态|SetisElevatorMoving false)))))))

(event EventMoveDownFloor
  ;[1 1 1] Elevator
  (if (and (< (Variables|State|GetElevatorState) 2) (not (Variables|状态|GetisElevatorMoving)))
    (Variables|状态|SetisElevatorMoving true)
    (Math|Integer|IncrementInt (Variables|State|GetElevatorState)
      (:%20%20
        (Utilities|StoreFloorTempLocation)
        (bind _goup (Timeline|FloorMoveDown PlayFromStart)
          (:Update
            (Utilities|AddFloorDeltaLocation (Math|Vector|MakeVector 0.0 0.0 _goup)))
          (:Finished
            (Variables|状态|SetisElevatorMoving false)))))))

(event EventChangeTimeSp
  (bind _defaultsceneroot (Variables|组件|GetDefaultSceneRoot))
  (bind _returnvalue (Transformation|GetWorldLocation _defaultsceneroot))
  ;[1 1 1] ChangeTime
  (bind _move (Timeline|TimeChange Play)
    (:Update
      (Transformation|SetWorldLocation _defaultsceneroot (Math|Vector|MakeVector (.x _returnvalue) _move (.z _returnvalue)) false false))))

(event EventSplitFloors
  (bind _回形馆_0elevator (Variables|Default|Get回形馆_0Elevator))
  ;[1 1 1] SplitFloors
  (if (not (Variables|状态|GetisElevatorMoving))
    (Utilities|WhileLoopwithDelay (> (Variables|State|GetElevatorState) 0) 1.0
      (:LoopBody
        (CallFunction|MoveUpFloor))
      (:Completed
        (Utilities|FlowControl|MultiGate false true -1
          (:Out%200
            (Variables|Default|SetSplitState 0)
            (bind (_direction _roof _floor3 _floor2) (Timeline|FloorSplit1 Play)
              (:Update
                (Utilities|SplitFloorbyDistance (Math|Vector|MakeVector (- 0.0 (stale _x)) (- 0.0 (stale _y)) (- _roof (stale _z))) (Math|Vector|MakeVector (stale _x) (- 0.0 (stale _y)) _floor3) (Math|Vector|MakeVector (- 0.0 (stale _x)) (stale _y) (+ _floor2 (stale _z))) (Math|Vector|MakeVector (stale _x) (stale _y) (+ (stale _z) (stale _z))) :!label _label))))
          (:Out%201
            (Variables|Default|SetSplitState 1)
            (Development|SetHiddeninGame _回形馆_0elevator true false)
            (bind (_direction_2 _x _y _z) (Timeline|FloorSplit2 Play)
              (:Update
                (goto _label))))
          (:Out%202
            (Variables|Default|SetSplitState 2)
            (Utilities|FlowControl|Sequence
              (:then_0
                (Timeline|FloorSplit1 Reverse))
              (:then_1
                (Timeline|FloorSplit2 Reverse))
              (:then_2
                (Utilities|FlowControl|Delay 1.5)
                (Development|SetHiddeninGame _回形馆_0elevator false false)))))))))

(event EventChangeTimeNormal
  (bind _defaultsceneroot (Variables|组件|GetDefaultSceneRoot))
  (bind _returnvalue (Transformation|GetWorldLocation _defaultsceneroot))
  ;[1 1 1] ChangeTime
  (bind _move (Timeline|TimeChange Reverse)
    (:Update
      (Transformation|SetWorldLocation _defaultsceneroot (Math|Vector|MakeVector (.x _returnvalue) _move (.z _returnvalue)) false false))))

(fn ConstructionScript
  (Utilities|FlowControl|Sequence
    (:then_0
      (bind _asgi_room_instance (Utilities|Casting|CastToGI_Room_Instance (Game|GetGameInstance)))
      (Variables|Reference|SetRoomInstanceRef _asgi_room_instance))
    (:then_1
      (Variables|组件|SetWalls (Utilities|Array|MakeArray (Variables|WallComps|Get回形馆_1FloorWall) (Variables|WallComps|Get回形馆_2FloorWall) (Variables|WallComps|Get回形馆_3FloorWall) (Variables|WallComps|Get回形馆_4RoofWall))))
    (:then_2
      (Variables|Default|SetInteractiveBoxes (Utilities|Array|MakeArray (Variables|BoxComps|GetFloor1Box) (Variables|Default|GetFloor1NBox) (Variables|Default|GetFloor1EBox) (Variables|BoxComps|GetFloor2Box) (Variables|Default|GetFloor2NWMBox) (Variables|Default|GetFloor2NWCBox) (Variables|Default|GetFloor2NEBox) (Variables|Default|GetFloor2EBox) (Variables|Default|GetFloor2SWMBox) (Variables|Default|GetFloor2SWCBox) (Variables|Default|GetFloor2SEBox) (Variables|BoxComps|GetFloor3Box) (Variables|Default|GetFloor3NWMBox) (Variables|Default|GetFloor3NWCBox) (Variables|Default|GetFloor3NEBox) (Variables|Default|GetFloor3EBox) (Variables|Default|GetFloor3SWMBox) (Variables|Default|GetFloor3SWCBox) (Variables|Default|GetFloor3SEBox) (Variables|BoxComps|GetFloor4Box))))))

(fn SetRelatedObjects
  (bind _asgi_room_instance (Utilities|Casting|CastToGI_Room_Instance (Game|GetGameInstance)))
  (Utilities|FlowControl|Sequence
    (:then_0
      ;[1 1 1] SetRelatedFloor
      (bind _asbp_interactive_basic (Utilities|Casting|CastToBP_Interactive_Basic (Variables|/Script/Engine.ChildActorComponent|GetChildActor (Variables|/Game/WorldInferRules/BP_Room_CubeHouse_S.BP_Room_CubeHouse_S_C|GetFloor1Box (Variables|/Game/WorldInferRules/GI_Room_Instance.GI_Room_Instance_C|GetcubeHouseS _asgi_room_instance)))))
      (bind _asbp_interactive_basic_2 (Utilities|Casting|CastToBP_Interactive_Basic (Variables|/Script/Engine.ChildActorComponent|GetChildActor (Variables|/Game/WorldInferRules/BP_Room_LightHouse_S.BP_Room_LightHouse_S_C|GetFloor1Box (Variables|/Game/WorldInferRules/GI_Room_Instance.GI_Room_Instance_C|GetlightHouseS _asgi_room_instance)))))
      (bind _asbp_interactive_basic_3 (Utilities|Casting|CastToBP_Interactive_Basic (Variables|/Script/Engine.ChildActorComponent|GetChildActor (Variables|BoxComps|GetFloor1Box))))
      (Variables|/Game/WorldInferRules/BP_Interactive_Basic.BP_Interactive_Basic_C|SetrelatedInteractive _asbp_interactive_basic_3 (Utilities|Array|MakeArray _asbp_interactive_basic))
      (Variables|/Game/WorldInferRules/BP_Interactive_Basic.BP_Interactive_Basic_C|SetrelatedInteractiveSp _asbp_interactive_basic_3 (Utilities|Array|MakeArray _asbp_interactive_basic_2)))
    (:then_1
      (bind _asbp_interactive_basic_4 (Utilities|Casting|CastToBP_Interactive_Basic (Variables|/Script/Engine.ChildActorComponent|GetChildActor (Variables|/Game/WorldInferRules/BP_Room_CubeHouse_S.BP_Room_CubeHouse_S_C|GetFloor2Box (Variables|/Game/WorldInferRules/GI_Room_Instance.GI_Room_Instance_C|GetcubeHouseS _asgi_room_instance)))))
      (bind _asbp_interactive_basic_5 (Utilities|Casting|CastToBP_Interactive_Basic (Variables|/Script/Engine.ChildActorComponent|GetChildActor (Variables|/Game/WorldInferRules/BP_Room_LightHouse_S.BP_Room_LightHouse_S_C|GetFloor2Box (Variables|/Game/WorldInferRules/GI_Room_Instance.GI_Room_Instance_C|GetlightHouseS _asgi_room_instance)))))
      (bind _asbp_interactive_basic_6 (Utilities|Casting|CastToBP_Interactive_Basic (Variables|/Script/Engine.ChildActorComponent|GetChildActor (Variables|BoxComps|GetFloor2Box))))
      (Variables|/Game/WorldInferRules/BP_Interactive_Basic.BP_Interactive_Basic_C|SetrelatedInteractive _asbp_interactive_basic_6 (Utilities|Array|MakeArray _asbp_interactive_basic_4))
      (Variables|/Game/WorldInferRules/BP_Interactive_Basic.BP_Interactive_Basic_C|SetrelatedInteractiveSp _asbp_interactive_basic_6 (Utilities|Array|MakeArray _asbp_interactive_basic_5)))
    (:then_2
      (bind _asbp_interactive_basic_7 (Utilities|Casting|CastToBP_Interactive_Basic (Variables|/Script/Engine.ChildActorComponent|GetChildActor (Variables|/Game/WorldInferRules/BP_Room_CubeHouse_S.BP_Room_CubeHouse_S_C|GetFloor3Box (Variables|/Game/WorldInferRules/GI_Room_Instance.GI_Room_Instance_C|GetcubeHouseS _asgi_room_instance)))))
      (bind _asbp_interactive_basic_8 (Utilities|Casting|CastToBP_Interactive_Basic (Variables|/Script/Engine.ChildActorComponent|GetChildActor (Variables|/Game/WorldInferRules/BP_Room_LightHouse_S.BP_Room_LightHouse_S_C|GetFloor3Box (Variables|/Game/WorldInferRules/GI_Room_Instance.GI_Room_Instance_C|GetlightHouseS _asgi_room_instance)))))
      (bind _asbp_interactive_basic_9 (Utilities|Casting|CastToBP_Interactive_Basic (Variables|/Script/Engine.ChildActorComponent|GetChildActor (Variables|BoxComps|GetFloor3Box))))
      (Variables|/Game/WorldInferRules/BP_Interactive_Basic.BP_Interactive_Basic_C|SetrelatedInteractive _asbp_interactive_basic_9 (Utilities|Array|MakeArray _asbp_interactive_basic_7))
      (Variables|/Game/WorldInferRules/BP_Interactive_Basic.BP_Interactive_Basic_C|SetrelatedInteractiveSp _asbp_interactive_basic_9 (Utilities|Array|MakeArray _asbp_interactive_basic_8)))
    (:then_3
      (bind _asbp_interactive_basic_10 (Utilities|Casting|CastToBP_Interactive_Basic (Variables|/Script/Engine.ChildActorComponent|GetChildActor (Variables|/Game/WorldInferRules/BP_Room_CubeHouse_S.BP_Room_CubeHouse_S_C|GetFloor4Box (Variables|/Game/WorldInferRules/GI_Room_Instance.GI_Room_Instance_C|GetcubeHouseS _asgi_room_instance)))))
      (bind _asbp_interactive_basic_11 (Utilities|Casting|CastToBP_Interactive_Basic (Variables|/Script/Engine.ChildActorComponent|GetChildActor (Variables|/Game/WorldInferRules/BP_Room_LightHouse_S.BP_Room_LightHouse_S_C|GetFloor4Box (Variables|/Game/WorldInferRules/GI_Room_Instance.GI_Room_Instance_C|GetlightHouseS _asgi_room_instance)))))
      (bind _asbp_interactive_basic_12 (Utilities|Casting|CastToBP_Interactive_Basic (Variables|/Script/Engine.ChildActorComponent|GetChildActor (Variables|BoxComps|GetFloor4Box))))
      (Variables|/Game/WorldInferRules/BP_Interactive_Basic.BP_Interactive_Basic_C|SetrelatedInteractive _asbp_interactive_basic_12 (Utilities|Array|MakeArray _asbp_interactive_basic_10))
      (Variables|/Game/WorldInferRules/BP_Interactive_Basic.BP_Interactive_Basic_C|SetrelatedInteractiveSp _asbp_interactive_basic_12 (Utilities|Array|MakeArray _asbp_interactive_basic_11)))
    (:then_4
      ;[1 1 1] SetRelatedRoom
      (bind _asbp_interactive_basic_13 (Utilities|Casting|CastToBP_Interactive_Basic (Variables|/Script/Engine.ChildActorComponent|GetChildActor (Variables|/Game/WorldInferRules/BP_Room_CubeHouse_S.BP_Room_CubeHouse_S_C|GetFloor1EBox (Variables|/Game/WorldInferRules/GI_Room_Instance.GI_Room_Instance_C|GetcubeHouseS _asgi_room_instance)))))
      (bind _asbp_interactive_basic_14 (Utilities|Casting|CastToBP_Interactive_Basic (Variables|/Script/Engine.ChildActorComponent|GetChildActor (Variables|/Game/WorldInferRules/BP_Room_LightHouse_S.BP_Room_LightHouse_S_C|GetFloor1WBox (Variables|/Game/WorldInferRules/GI_Room_Instance.GI_Room_Instance_C|GetlightHouseS _asgi_room_instance)))))
      (bind _asbp_interactive_basic_15 (Utilities|Casting|CastToBP_Interactive_Basic (Variables|/Script/Engine.ChildActorComponent|GetChildActor (Variables|Default|GetFloor1EBox))))
      (Variables|/Game/WorldInferRules/BP_Interactive_Basic.BP_Interactive_Basic_C|SetrelatedInteractive _asbp_interactive_basic_15 (Utilities|Array|MakeArray _asbp_interactive_basic_13))
      (Variables|/Game/WorldInferRules/BP_Interactive_Basic.BP_Interactive_Basic_C|SetrelatedInteractiveSp _asbp_interactive_basic_15 (Utilities|Array|MakeArray _asbp_interactive_basic_14)))
    (:then_5
      (bind _asbp_interactive_basic_16 (Utilities|Casting|CastToBP_Interactive_Basic (Variables|/Script/Engine.ChildActorComponent|GetChildActor (Variables|/Game/WorldInferRules/BP_Room_CubeHouse_S.BP_Room_CubeHouse_S_C|GetFloor2EBox (Variables|/Game/WorldInferRules/GI_Room_Instance.GI_Room_Instance_C|GetcubeHouseS _asgi_room_instance)))))
      (bind _asbp_interactive_basic_17 (Utilities|Casting|CastToBP_Interactive_Basic (Variables|/Script/Engine.ChildActorComponent|GetChildActor (Variables|Default|GetFloor2EBox))))
      (Variables|/Game/WorldInferRules/BP_Interactive_Basic.BP_Interactive_Basic_C|SetrelatedInteractive _asbp_interactive_basic_17 (Utilities|Array|MakeArray _asbp_interactive_basic_16)))
    (:then_6
      (bind _asbp_interactive_basic_18 (Utilities|Casting|CastToBP_Interactive_Basic (Variables|/Script/Engine.ChildActorComponent|GetChildActor (Variables|/Game/WorldInferRules/BP_Room_CubeHouse_S.BP_Room_CubeHouse_S_C|GetFloor3EBox (Variables|/Game/WorldInferRules/GI_Room_Instance.GI_Room_Instance_C|GetcubeHouseS _asgi_room_instance)))))
      (bind _asbp_interactive_basic_19 (Utilities|Casting|CastToBP_Interactive_Basic (Variables|/Script/Engine.ChildActorComponent|GetChildActor (Variables|Default|GetFloor3EBox))))
      (Variables|/Game/WorldInferRules/BP_Interactive_Basic.BP_Interactive_Basic_C|SetrelatedInteractive _asbp_interactive_basic_19 (Utilities|Array|MakeArray _asbp_interactive_basic_18)))))