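; Lighthouse room actor for a time-switching puzzle house, with interactive floor boxes linked to LightHouseM and CubeHouseM counterparts.
; Timelines drive wall fading through dynamic materials assigned at BeginPlay, staged house separation, and two-step floor splitting.
; Splitting first lowers a fake, delay-based elevator counter to zero; its second step undoes any separation and blocks further separation.
; Time-change events toggle visibility and interactivity, slide the root along Y, and mirror the tower room for CubeHouse.
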(event Custom|HideWalls
  ;[1 1 1] HideWalls
  (bind _isa (Utilities|FlowControl|FlipFlop)
    (:A
      (bind _fade (Timeline|WallsFade Play)
        (:Update
          (Rendering|Material|SetScalarParameterValue (Variables|WallDynamicMaterial|GetDynamicBrickMat) "FadeAmount" _fade :!class /Script/Engine.MaterialInstanceDynamic)
          (Rendering|Material|SetScalarParameterValue (Variables|WallDynamicMaterial|GetDynamicConcreteMat) "FadeAmount" _fade :!class /Script/Engine.MaterialInstanceDynamic)
          (Rendering|Material|SetScalarParameterValue (Variables|WallDynamicMaterial|GetDynamicWoodMat) "FadeAmount" _fade :!class /Script/Engine.MaterialInstanceDynamic)
          (Rendering|Material|SetScalarParameterValue (Variables|WallDynamicMaterial|GetDynamicRoofMat) "FadeAmount" _fade :!class /Script/Engine.MaterialInstanceDynamic)
          (Rendering|Material|SetScalarParameterValue (Variables|WallDynamicMaterial|GetDynamicRoofMat2) "FadeAmount" _fade :!class /Script/Engine.MaterialInstanceDynamic))
        (:Finished
          (Variables|Default|SetisWallsHide _isa))))
    (:B
      (Timeline|WallsFade Reverse))))

(event Custom|SecondCaseStart
  (Development|SetHiddeninGame (Variables|Default|Get时之灯塔_0FloorS) false false))

(event EventBeginPlay
  (Utilities|FlowControl|Sequence
    (:then_0
      (bind _asgi_room_instance (Utilities|Casting|CastToGI_Room_Instance (Game|GetGameInstance)))
      (Variables|Reference|SetRoomInstanceRef _asgi_room_instance))
    (:then_1
      (Utilities|DamagedMaterialSolve))))

(event EventMoveUpFloor
  ;[1 1 1] Elevator(Fake)
  (if (and (> (Variables|状态|GetElevatorState) 0) (not (Variables|状态|GetisElevatorMoving)))
    (Variables|状态|SetisElevatorMoving true)
    (Math|Integer|DecrementInt (Variables|状态|GetElevatorState)
      (:%20%20
        (Utilities|FlowControl|Delay 1.0)
        (Variables|状态|SetisElevatorMoving false)))))

(event EventMoveDownFloor
  ;[1 1 1] Elevator(Fake)
  (if (and (< (Variables|状态|GetElevatorState) 2) (not (Variables|状态|GetisElevatorMoving)))
    (Variables|状态|SetisElevatorMoving true)
    (Math|Integer|IncrementInt (Variables|状态|GetElevatorState)
      (:%20%20
        (Utilities|FlowControl|Delay 1.0)
        (Variables|状态|SetisElevatorMoving false)))))

(event EventChangeTimeSp
  (bind _self self)
  (bind _defaultsceneroot (Variables|组件|GetDefaultSceneRoot))
  (bind _returnvalue (Transformation|GetWorldLocation _defaultsceneroot))
  (bind _bhidden (Variables|Default|GetbHidden _self))
  (bind _returnvalue_2 (not _bhidden))
  ;[1 1 1] ChangeTime
  (if (Variables|/Game/WorldInferRules/GI_Room_Instance.GI_Room_Instance_C|GetisCubeHouseSp (Variables|Reference|GetRoomInstanceRef))
    (Transformation|SetRelativeScale3D (Variables|Default|Get时之灯塔_TowerRoomS) "1.000000,-1.000000,1.000000"))
  (Rendering|SetActorHiddenInGame _returnvalue_2)
  (CallFunction|MovetoHide _bhidden)
  (CallFunction|EnableInteractive _returnvalue_2)
  (Development|SetHiddeninGame (Variables|Default|Get时之灯塔_TowerRoomS) false true)
  (bind _move (Timeline|TimeChange1 PlayFromStart)
    (:Update
      (Transformation|SetWorldLocation _defaultsceneroot (Math|Vector|MakeVector (.x _returnvalue) _move (.z _returnvalue)) false false))))

(event EventSplitFloors
  (bind _sepcontainer (Variables|ContainerComps|GetSepContainer))
  (bind _relativelocation (Variables|/Script/Engine.SceneComponent|GetRelativeLocation _sepcontainer))
  ;[1 1 1] SplitFloors
  (if (not (Variables|状态|GetisElevatorMoving))
    (Utilities|WhileLoopwithDelay (> (Variables|状态|GetElevatorState) 0) 1.0
      (:LoopBody
        (CallFunction|MoveUpFloor))
      (:Completed
        (Utilities|FlowControl|MultiGate false true -1
          (:Out%200
            (Variables|Default|SetSplitState 0)
            (bind (_direction _roof _floor3 _floor2) (Timeline|FloorSplit1 Play)
              (:Update
                (Utilities|SplitFloorbyDistance (Math|Vector|MakeVector (- 0.0 (stale _x)) (- 0.0 (stale _y)) (- _roof (stale _z))) (Math|Vector|MakeVector (stale _x) (- 0.0 (stale _y)) _floor3) (Math|Vector|MakeVector (- 0.0 (stale _x)) (stale _y) (+ _floor2 (stale _z))) (Math|Vector|MakeVector (stale _x) (stale _y) (+ (stale _z) (stale _z))) :!label _label))))
          (:Out%201
            (Variables|Default|SetSplitState 1)
            (Utilities|FlowControl|Sequence
              (:then_0
                ;[1 1 1] SeparateHouse
                (switch int (Variables|State|GetSeparateState)
                  (:0
                    (Utilities|FlowControl|Sequence
                      (:then_0
                        (Utilities|FlowControl|MultiGate false true -1) ; enters at Reset
                      )
                      (:then_1
                        (bind _angle (Timeline|HouseSeparate1 Reverse)
                          (:Update
                            (Transformation|SetRelativeRotation (Variables|ContainerComps|GetSepContainer) (Math|Rotator|MakeRotator 0.0 0.0 _angle) false false))))))
                  (:1
                    (Utilities|FlowControl|Sequence
                      (:then_0
                        (Utilities|FlowControl|MultiGate false true -1) ; enters at Reset
                      )
                      (:then_1
                        (Utilities|FlowControl|Sequence
                          (:then_0
                            (Timeline|HouseSeparate1 Reverse))
                          (:then_1
                            (bind _distance (Timeline|HouseSeparate2 Reverse)
                              (:Update
                                (Transformation|SetRelativeLocation _sepcontainer (Math|Vector|MakeVector _distance (.y _relativelocation) (.z _relativelocation)) false false))))))))))
              (:then_1
                (bind (_direction_2 _x _y _z) (Timeline|FloorSplit2 Play)
                  (:Update
                    (goto _label))))))
          (:Out%202
            (Variables|Default|SetSplitState 2)
            (Utilities|FlowControl|Sequence
              (:then_0
                (Timeline|FloorSplit1 Reverse))
              (:then_1
                (Timeline|FloorSplit2 Reverse)))))))))

(event EventChangeTimeNormal
  (bind _self self)
  (bind _defaultsceneroot (Variables|组件|GetDefaultSceneRoot))
  (bind _returnvalue (Transformation|GetWorldLocation _defaultsceneroot))
  (bind _bhidden (Variables|Default|GetbHidden _self))
  (bind _returnvalue_2 (not _bhidden))
  ;[1 1 1] ChangeTime
  (Transformation|SetRelativeScale3D (Variables|Default|Get时之灯塔_TowerRoomS) "1.000000,1.000000,1.000000")
  (Rendering|SetActorHiddenInGame _returnvalue_2)
  (CallFunction|MovetoHide _bhidden)
  (CallFunction|EnableInteractive _returnvalue_2)
  (Development|SetHiddeninGame (Variables|Default|Get时之灯塔_TowerRoomS) true true)
  (bind _move (Timeline|TimeChange2 ReverseFromEnd)
    (:Update
      (Transformation|SetWorldLocation _defaultsceneroot (Math|Vector|MakeVector (.x _returnvalue) _move (.z _returnvalue)) false false))))

(event EventSeparateHouse
  (bind _sepcontainer (Variables|ContainerComps|GetSepContainer))
  (bind _relativelocation (Variables|/Script/Engine.SceneComponent|GetRelativeLocation _sepcontainer))
  ;[1 1 1] SeparateHouse
  (if (!= (Variables|Default|GetSplitState) 1)
    (Utilities|FlowControl|MultiGate false true -1
      (:Out%200
        (Variables|State|SetSeparateState 0)
        (bind _angle (Timeline|HouseSeparate1 Play)
          (:Update
            (Transformation|SetRelativeRotation (Variables|ContainerComps|GetSepContainer) (Math|Rotator|MakeRotator 0.0 0.0 _angle) false false))))
      (:Out%201
        (Variables|State|SetSeparateState 1)
        (bind _distance (Timeline|HouseSeparate2 Play)
          (:Update
            (Transformation|SetRelativeLocation _sepcontainer (Math|Vector|MakeVector _distance (.y _relativelocation) (.z _relativelocation)) false false))))
      (:Out%202
        (Variables|State|SetSeparateState 2)
        (Utilities|FlowControl|Sequence
          (:then_0
            (Timeline|HouseSeparate1 Reverse))
          (:then_1
            (Timeline|HouseSeparate2 Reverse)))))))

(fn ConstructionScript
  (Utilities|FlowControl|Sequence
    (:then_1
      (Variables|Default|SetInteractiveBoxes (Utilities|Array|MakeArray (Variables|BoxComps|GetFloor1Box) (Variables|Default|GetFloor1NBox) (Variables|Default|GetFloor1NEBox) (Variables|Default|GetFloor1WBox) (Variables|Default|GetFloor1EBox) (Variables|Default|GetFloor1SBox) (Variables|BoxComps|GetFloor2Box) (Variables|Default|GetFloor2NBox) (Variables|Default|GetFloor2NEBox) (Variables|Default|GetFloor2EBox) (Variables|Default|GetFloor2SBox) (Variables|BoxComps|GetFloor3Box) (Variables|Default|GetFloor4Box))))))

(fn SetRelatedObjects
  (bind _asgi_room_instance (Utilities|Casting|CastToGI_Room_Instance (Game|GetGameInstance)))
  (Utilities|FlowControl|Sequence
    (:then_0
      ;[1 1 1] SetRelatedFloor
      (bind _asbp_interactive_basic (Utilities|Casting|CastToBP_Interactive_Basic (Variables|/Script/Engine.ChildActorComponent|GetChildActor (Variables|/Game/WorldInferRules/BP_Room_LightHouse_M.BP_Room_LightHouse_M_C|GetFloor1Box (Variables|/Game/WorldInferRules/GI_Room_Instance.GI_Room_Instance_C|GetlightHouseM _asgi_room_instance)))))
      (bind _asbp_interactive_basic_2 (Utilities|Casting|CastToBP_Interactive_Basic (Variables|/Script/Engine.ChildActorComponent|GetChildActor (Variables|/Game/WorldInferRules/BP_Room_CubeHouse_M.BP_Room_CubeHouse_M_C|GetFloor1Box (Variables|/Game/WorldInferRules/GI_Room_Instance.GI_Room_Instance_C|GetcubeHouseM _asgi_room_instance)))))
      (bind _asbp_interactive_basic_3 (Utilities|Casting|CastToBP_Interactive_Basic (Variables|/Script/Engine.ChildActorComponent|GetChildActor (Variables|BoxComps|GetFloor1Box))))
      (Variables|/Game/WorldInferRules/BP_Interactive_Basic.BP_Interactive_Basic_C|SetrelatedInteractive _asbp_interactive_basic_3 (Utilities|Array|MakeArray _asbp_interactive_basic))
      (Variables|/Game/WorldInferRules/BP_Interactive_Basic.BP_Interactive_Basic_C|SetrelatedInteractiveSp _asbp_interactive_basic_3 (Utilities|Array|MakeArray _asbp_interactive_basic_2)))
    (:then_1
      (bind _asbp_interactive_basic_4 (Utilities|Casting|CastToBP_Interactive_Basic (Variables|/Script/Engine.ChildActorComponent|GetChildActor (Variables|/Game/WorldInferRules/BP_Room_LightHouse_M.BP_Room_LightHouse_M_C|GetFloor2Box (Variables|/Game/WorldInferRules/GI_Room_Instance.GI_Room_Instance_C|GetlightHouseM _asgi_room_instance)))))
      (bind _asbp_interactive_basic_5 (Utilities|Casting|CastToBP_Interactive_Basic (Variables|/Script/Engine.ChildActorComponent|GetChildActor (Variables|/Game/WorldInferRules/BP_Room_CubeHouse_M.BP_Room_CubeHouse_M_C|GetFloor2Box (Variables|/Game/WorldInferRules/GI_Room_Instance.GI_Room_Instance_C|GetcubeHouseM _asgi_room_instance)))))
      (bind _asbp_interactive_basic_6 (Utilities|Casting|CastToBP_Interactive_Basic (Variables|/Script/Engine.ChildActorComponent|GetChildActor (Variables|BoxComps|GetFloor2Box))))
      (Variables|/Game/WorldInferRules/BP_Interactive_Basic.BP_Interactive_Basic_C|SetrelatedInteractive _asbp_interactive_basic_6 (Utilities|Array|MakeArray _asbp_interactive_basic_4))
      (Variables|/Game/WorldInferRules/BP_Interactive_Basic.BP_Interactive_Basic_C|SetrelatedInteractiveSp _asbp_interactive_basic_6 (Utilities|Array|MakeArray _asbp_interactive_basic_5)))
    (:then_2
      (bind _asbp_interactive_basic_7 (Utilities|Casting|CastToBP_Interactive_Basic (Variables|/Script/Engine.ChildActorComponent|GetChildActor (Variables|/Game/WorldInferRules/BP_Room_LightHouse_M.BP_Room_LightHouse_M_C|GetFloor3Box (Variables|/Game/WorldInferRules/GI_Room_Instance.GI_Room_Instance_C|GetlightHouseM _asgi_room_instance)))))
      (bind _asbp_interactive_basic_8 (Utilities|Casting|CastToBP_Interactive_Basic (Variables|/Script/Engine.ChildActorComponent|GetChildActor (Variables|/Game/WorldInferRules/BP_Room_CubeHouse_M.BP_Room_CubeHouse_M_C|GetFloor3Box (Variables|/Game/WorldInferRules/GI_Room_Instance.GI_Room_Instance_C|GetcubeHouseM _asgi_room_instance)))))
      (bind _asbp_interactive_basic_9 (Utilities|Casting|CastToBP_Interactive_Basic (Variables|/Script/Engine.ChildActorComponent|GetChildActor (Variables|BoxComps|GetFloor3Box))))
      (Variables|/Game/WorldInferRules/BP_Interactive_Basic.BP_Interactive_Basic_C|SetrelatedInteractive _asbp_interactive_basic_9 (Utilities|Array|MakeArray _asbp_interactive_basic_7))
      (Variables|/Game/WorldInferRules/BP_Interactive_Basic.BP_Interactive_Basic_C|SetrelatedInteractiveSp _asbp_interactive_basic_9 (Utilities|Array|MakeArray _asbp_interactive_basic_8)))
    (:then_3
      (bind _asbp_interactive_basic_10 (Utilities|Casting|CastToBP_Interactive_Basic (Variables|/Script/Engine.ChildActorComponent|GetChildActor (Variables|/Game/WorldInferRules/BP_Room_LightHouse_M.BP_Room_LightHouse_M_C|GetFloor4Box (Variables|/Game/WorldInferRules/GI_Room_Instance.GI_Room_Instance_C|GetlightHouseM _asgi_room_instance)))))
      (bind _asbp_interactive_basic_11 (Utilities|Casting|CastToBP_Interactive_Basic (Variables|/Script/Engine.ChildActorComponent|GetChildActor (Variables|/Game/WorldInferRules/BP_Room_CubeHouse_M.BP_Room_CubeHouse_M_C|GetFloor4Box (Variables|/Game/WorldInferRules/GI_Room_Instance.GI_Room_Instance_C|GetcubeHouseM _asgi_room_instance)))))
      (bind _asbp_interactive_basic_12 (Utilities|Casting|CastToBP_Interactive_Basic (Variables|/Script/Engine.ChildActorComponent|GetChildActor (Variables|Default|GetFloor4Box))))
      (Variables|/Game/WorldInferRules/BP_Interactive_Basic.BP_Interactive_Basic_C|SetrelatedInteractive _asbp_interactive_basic_12 (Utilities|Array|MakeArray _asbp_interactive_basic_10))
      (Variables|/Game/WorldInferRules/BP_Interactive_Basic.BP_Interactive_Basic_C|SetrelatedInteractiveSp _asbp_interactive_basic_12 (Utilities|Array|MakeArray _asbp_interactive_basic_11)))
    (:then_4
      ;[1 1 1] SetRelatedRoom
      (bind _asbp_interactive_basic_13 (Utilities|Casting|CastToBP_Interactive_Basic (Variables|/Script/Engine.ChildActorComponent|GetChildActor (Variables|/Game/WorldInferRules/BP_Room_CubeHouse_M.BP_Room_CubeHouse_M_C|GetFloor1EBox (Variables|/Game/WorldInferRules/GI_Room_Instance.GI_Room_Instance_C|GetcubeHouseM _asgi_room_instance)))))
      (bind _asbp_interactive_basic_14 (Utilities|Casting|CastToBP_Interactive_Basic (Variables|/Script/Engine.ChildActorComponent|GetChildActor (Variables|Default|GetFloor1WBox))))
      (Variables|/Game/WorldInferRules/BP_Interactive_Basic.BP_Interactive_Basic_C|SetrelatedInteractiveSp _asbp_interactive_basic_14 (Utilities|Array|MakeArray _asbp_interactive_basic_13)))))