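; Player controller for the room scene that spawns and possesses an orbit camera, adds UI widgets and registers itself with GI_Room_Instance.
; Mouse and touch inputs rotate with clamped pitch and zoom within the current object level's arm range.
; Zooming out past that range or quick right-clicking calls UpdateClickedObject on the game instance.
; Timelines interpolate the camera between object levels, reattaching it afterwards, and to set rotations such as top-down view.
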(event Custom|UpdateCameraPosition
  (params (ObjectLevel :type Integer) (NewParent :type Scene%20Component%20Object%20Reference))
  (bind _roominstanceref (Variables|Reference|GetroomInstanceRef))
  (bind _cameraarmlength (Variables|/Game/WorldInferRules/GI_Room_Instance.GI_Room_Instance_C|GetcameraArmLength _roominstanceref))
  (bind _output (Utilities|Array|Get(acopy) _cameraarmlength ObjectLevel))
  ;[1 1 1] CameraUpdate
  (Variables|Private|SetcameraLocationTemp (Transformation|GetActorLocation (Variables|Reference|GetroomCameraRef)))
  (Variables|Private|SetcameraArmLengthTemp (Variables|/Script/Engine.SpringArmComponent|GetTargetArmLength (Variables|/Game/WorldInferRules/BP_RoomCamera.BP_RoomCamera_C|GetSpringArm (Variables|Reference|GetroomCameraRef))))
  (if (> _output (Variables|Default|GetmaxArm))
    (Variables|Default|SetmaxArm _output)
    (bind _move1 (Timeline|cameraMove PlayFromStart)
      (:Update
        (Utilities|UpdateCameraPositionTick NewParent _move1 _output))
      (:Finished
        (Utilities|UpdateCameraPositionPost (Utilities|Array|Get(acopy) _cameraarmlength (+ ObjectLevel 1)) _output NewParent)))
    (else
      (Timeline|cameraMove PlayFromStart))))

(event Custom|CameraGodVision
  (bind _returnvalue (Pawn|GetControlRotation :!class /Script/Engine.Controller))
  ;[1 1 1] GodVision
  (Variables|Default|SetCameraTargetRotationTemp "-90.000000,0.000000,0.000000")
  (bind _output_get (Variables|Default|SetCameraOriginRotationTemp (Math|Rotator|MakeRotator 0.0 (Math|Float|SelectFloat (- (.pitch _returnvalue) 3.6e+02) (.pitch _returnvalue) (> (.pitch _returnvalue) 0.0)) (.yaw _returnvalue))))
  (bind _move1 (Timeline|CameraMove2 PlayFromStart)
    (:Update
      (Pawn|SetControlRotation (Math|Rotator|MakeRotator 0.0 (Utilities|CalcDeltaDist (.pitch (Variables|Default|GetCameraTargetRotationTemp)) (.pitch _output_get) _move1) (Utilities|CalcDeltaDist (.yaw (Variables|Default|GetCameraTargetRotationTemp)) (.yaw _output_get) _move1))))))

(event Custom|SetCameraRotation
  (params (NewParam :type Rotator))
  (bind _returnvalue (Pawn|GetControlRotation :!class /Script/Engine.Controller))
  ;[1 1 1] GodVision
  (Variables|Default|SetCameraTargetRotationTemp NewParam)
  (bind _output_get (Variables|Default|SetCameraOriginRotationTemp (Math|Rotator|MakeRotator 0.0 (Math|Float|SelectFloat (- (.pitch _returnvalue) 3.6e+02) (.pitch _returnvalue) (> (.pitch _returnvalue) 0.0)) (.yaw _returnvalue))))
  (bind _move1 (Timeline|CameraMove2 PlayFromStart)
    (:Update
      (Pawn|SetControlRotation (Math|Rotator|MakeRotator 0.0 (Utilities|CalcDeltaDist (.pitch (Variables|Default|GetCameraTargetRotationTemp)) (.pitch _output_get) _move1) (Utilities|CalcDeltaDist (.yaw (Variables|Default|GetCameraTargetRotationTemp)) (.yaw _output_get) _move1))))))

(event Input|EnhancedActionEvents|EnhancedInputActionIA_RoomRotate_Touch
  (params (ActionValue :type Vector%202D%20Structure) (ElapsedSeconds :type Float%20%28double-precision%29) (TriggeredSeconds :type Float%20%28double-precision%29) (InputAction :type Input%20Action%20Object%20Reference :default "/Game/WorldInferRules/Inputs/IA_RoomRotate_Touch.IA_RoomRotate_Touch"))
  (bind _roomcameraref (Variables|Reference|GetroomCameraRef))
  (bind _returnvalue (Pawn|GetControlRotation _roomcameraref :!class /Script/Engine.Pawn))
  (bind (_roll _pitch _yaw) (Math|Rotator|BreakRotator _returnvalue))
  ;[1 1 1] CameraRotate
  (:Triggered
    (Utilities|FlowControl|Sequence
      (:then_0
        (Pawn|Input|AddControllerYawInput (Variables|Reference|GetroomCameraRef) (* (.x (- ActionValue (Variables|Default|GetoldTouchLocation))) 0.2)))
      (:then_1
        (Pawn|SetControlRotation (Math|Rotator|MakeRotator _roll (Math|Float|ClampAngle (+ _pitch (* (.y (- ActionValue (Variables|Default|GetoldTouchLocation))) -0.2)) -9e+01 0.0) _yaw)))
      (:then_2
        (Variables|Default|SetoldTouchLocation ActionValue :!label _label))))
  (:Started
    (goto _label)))

(event Input|EnhancedActionEvents|EnhancedInputActionIA_RoomZoom
  (params (ActionValue :type Float%20%28double-precision%29) (ElapsedSeconds :type Float%20%28double-precision%29) (TriggeredSeconds :type Float%20%28double-precision%29) (InputAction :type Input%20Action%20Object%20Reference :default "/Game/WorldInferRules/Inputs/IA_RoomZoom.IA_RoomZoom"))
  (bind _roomcameraref (Variables|Reference|GetroomCameraRef))
  (bind _armlenstep (Variables|Default|GetarmLenStep))
  (bind _returnvalue (* ActionValue _armlenstep))
  (bind _springarm (Variables|/Game/WorldInferRules/BP_RoomCamera.BP_RoomCamera_C|GetSpringArm _roomcameraref))
  ;[1 1 1] CameraZoom
  ;;[1 1 1] Mouse
  (if (and (> _returnvalue 0.0) (== (Variables|/Script/Engine.SpringArmComponent|GetTargetArmLength _springarm) (Variables|Default|GetmaxArm)))
    (Default|UpdateClickedObject (Variables|Reference|GetroomInstanceRef))
    (else
      (Variables|/Script/Engine.SpringArmComponent|SetTargetArmLength _springarm (Math|Float|Clamp(Float) (+ _returnvalue (Variables|/Script/Engine.SpringArmComponent|GetTargetArmLength _springarm)) (Variables|Default|GetminArm) (Variables|Default|GetmaxArm))))))

(event Input|EnhancedActionEvents|EnhancedInputActionIA_RoomRotate
  (params (ActionValue :type Vector%202D%20Structure) (ElapsedSeconds :type Float%20%28double-precision%29) (TriggeredSeconds :type Float%20%28double-precision%29) (InputAction :type Input%20Action%20Object%20Reference :default "/Game/WorldInferRules/Inputs/IA_RoomRotate.IA_RoomRotate"))
  (bind _roomcameraref (Variables|Reference|GetroomCameraRef))
  (bind _returnvalue (Pawn|GetControlRotation _roomcameraref :!class /Script/Engine.Pawn))
  (bind (_roll _pitch _yaw) (Math|Rotator|BreakRotator _returnvalue))
  ;[1 1 1] CameraRotate
  (Utilities|FlowControl|Sequence
    (:then_0
      (Pawn|Input|AddControllerYawInput (Variables|Reference|GetroomCameraRef) (* (.x ActionValue) 2.0)))
    (:then_1
      (Pawn|SetControlRotation (Math|Rotator|MakeRotator _roll (Math|Float|ClampAngle (+ (* (.y ActionValue) 2.0) _pitch) -9e+01 0.0) _yaw)))))

(event Input|EnhancedActionEvents|EnhancedInputActionIA_RoomZoom_Touch
  (params (ActionValue :type Float%20%28double-precision%29) (ElapsedSeconds :type Float%20%28double-precision%29) (TriggeredSeconds :type Float%20%28double-precision%29) (InputAction :type Input%20Action%20Object%20Reference :default "/Game/WorldInferRules/Inputs/IA_RoomZoom_Touch.IA_RoomZoom_Touch"))
  (bind _roomcameraref (Variables|Reference|GetroomCameraRef))
  (bind _springarm (Variables|/Game/WorldInferRules/BP_RoomCamera.BP_RoomCamera_C|GetSpringArm _roomcameraref))
  ;[1 1 1] CameraZoom
  ;;[1 1 1] Touch
  (:Triggered
    (if (Variables|Default|GetisFirstSqueeze)
      (if (and (== (stale _output_get) (Variables|Default|GetmaxArm)) (< ActionValue 1.0))
        (Utilities|FlowControl|Sequence
          (:then_0
            (Default|UpdateClickedObject (Variables|Reference|GetroomInstanceRef)))
          (:then_1
            (CallFunction|AddDebugMessage "squeezeOut")))
        (else
          (Utilities|FlowControl|Sequence
            (:then_0
              (Variables|Default|SetisFirstSqueeze (== ActionValue 1.0))
              (Variables|/Script/Engine.SpringArmComponent|SetTargetArmLength _springarm (Math|Float|Clamp(Float) (* (Variables|Private|GetarmLengthTouchTemp) (Math|Float|Sqrt (Math|Float|Sqrt (/ 1.0 ActionValue)))) (Variables|Default|GetminArm) (Variables|Default|GetmaxArm)) :!label _label))
            (:then_1
              (CallFunction|AddDebugMessage (Class|KismetStringLibrary|BuildStringDouble "armLen = " "" (Math|Float|Clamp(Float) (* (Variables|Private|GetarmLengthTouchTemp) (Math|Float|Sqrt (Math|Float|Sqrt (/ 1.0 ActionValue)))) (Variables|Default|GetminArm) (Variables|Default|GetmaxArm))) :!label _label_2)))))
      (else
        (Utilities|FlowControl|Sequence
          (:then_0
            (goto _label))
          (:then_1
            (goto _label_2))))))
  (:Started
    (bind _output_get (Variables|Private|SetarmLengthTouchTemp (Variables|/Script/Engine.SpringArmComponent|GetTargetArmLength _springarm)))
    (Variables|Default|SetisFirstSqueeze true)
    (CallFunction|AddDebugMessage "isFirstSqueeze")))

(event EventBeginPlay
  (Utilities|FlowControl|Sequence
    (:then_0
      (Input|AddMappingContext (PlayerController|LocalPlayerSubsystems|GetEnhancedInputLocalPlayerSubsystem self) "/Game/WorldInferRules/Inputs/IC_RoomInputMap.IC_RoomInputMap" 0 "(bIgnoreAllPressedKeysUntilRelease=True,bForceImmediately=False,bNotifyUserSettings=False)"))
    (:then_1
      (bind _returnvalue (Game|SpawnActorfromClass "/Game/WorldInferRules/BP_RoomCamera.BP_RoomCamera_C" (Math|Transform|MakeTransform (Variables|/Game/WorldInferRules/GI_Room_Instance.GI_Room_Instance_C|GetcameraInitLocation (Variables|Reference|GetroomInstanceRef))) "Undefined" "MultiplyWithRoot" 0 0))
      (bind _output_get (Variables|Reference|SetroomCameraRef _returnvalue))
      (Variables|/Script/Engine.SpringArmComponent|SetTargetArmLength (Variables|/Game/WorldInferRules/BP_RoomCamera.BP_RoomCamera_C|GetSpringArm _output_get) (Utilities|Array|Get(acopy) (Variables|/Game/WorldInferRules/GI_Room_Instance.GI_Room_Instance_C|GetcameraArmLength (Variables|Reference|GetroomInstanceRef))))
      (Pawn|Possess _output_get))
    (:then_2
      (bind _returnvalue_2 (UserInterface|CreateWidget "/Game/WorldInferRules/UMG/UW_MainScreenUI.UW_MainScreenUI_C"))
      (UserInterface|Viewport|AddtoViewport _returnvalue_2 0))
    (:then_3
      (bind _returnvalue_3 (UserInterface|CreateWidget "/Game/WorldInferRules/UMG/UW_TipText.UW_TipText_C"))
      (bind _output_get_2 (Variables|Reference|SettipWidgetRef _returnvalue_3))
      (UserInterface|Viewport|AddtoViewport _output_get_2 0))
    (:then_4
      (bind _returnvalue_4 (UserInterface|CreateWidget "/Game/WorldInferRules/UMG/SoundControl.SoundControl_C"))
      (UserInterface|Viewport|AddtoViewport _returnvalue_4 0))))

(event Input|MouseEvents|RightMouseButton
  (params (Key :type Key%20Structure :default "None"))
  (bind _returnvalue (Utilities|Time|GetGameTimeinSeconds))
  ;[1 1 1] CameraZoom
  (:Pressed
    (bind _output_get (Variables|Private|SetrightClickTimeTemp _returnvalue)))
  (:Released
    (if (< (- _returnvalue _output_get) 0.3)
      (Default|UpdateClickedObject (Variables|Reference|GetroomInstanceRef)))))

(fn ConstructionScript
  (bind _asgi_room_instance (Utilities|Casting|CastToGI_Room_Instance (Game|GetGameInstance)))
  (bind _output_get (Variables|Reference|SetroomInstanceRef _asgi_room_instance))
  (Variables|/Game/WorldInferRules/GI_Room_Instance.GI_Room_Instance_C|SetroomControllerRef _output_get self)
  (Variables|Default|SetmaxArm (Utilities|Array|Get(acopy) (Variables|/Game/WorldInferRules/GI_Room_Instance.GI_Room_Instance_C|GetcameraArmLength _output_get)))
  (Variables|Default|SetminArm (Utilities|Array|Get(acopy) (Variables|/Game/WorldInferRules/GI_Room_Instance.GI_Room_Instance_C|GetcameraArmLength _output_get) 1)))

(fn AddDebugMessage
  (params (A :type String))
  (bind _debugwidgetref (Variables|Reference|GetdebugWidgetRef))
  (bind _textblock (Variables|/Game/WorldInferRules/UMG/UW_DebugPrint.UW_DebugPrint_C|GetTextBlock _debugwidgetref))
  (Development|PrintString A)
  (Utilities|IsValid _debugwidgetref
    (:Is%20Valid
      (Rendering|Components|TextRender|SetText _textblock (Utilities|Text|ToText(String) (Utilities|String|Append A " 
" (Utilities|String|ToString(Text) (Variables|/Script/UMG.TextBlock|GetText _textblock))))))))

(fn ShowTipText
  (params (InText :type String))
  (Default|ShowTipText (Variables|Reference|GettipWidgetRef) InText))

(fn EnableDebugWidget
  (params (Condition :type Boolean))
  (Utilities|IsValid (Variables|Reference|GetdebugWidgetRef)
    (:Is%20Valid
      (if Condition
        (UserInterface|Viewport|AddtoViewport (stale _output_get) 0 :!label _label)
        (else
          (Widget|RemovefromParent (Variables|Reference|GetdebugWidgetRef)))))
    (:Is%20Not%20Valid
      (if Condition
        (bind _returnvalue (UserInterface|CreateWidget "/Game/WorldInferRules/UMG/UW_DebugPrint.UW_DebugPrint_C" self))
        (bind _output_get (Variables|Reference|SetdebugWidgetRef _returnvalue))
        (goto _label)))))