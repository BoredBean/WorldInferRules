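; Lighthouse puzzle room actor that animates the building and stages its cases up to the final trick.
; Timelines fade walls via dynamic materials, cycle exploded floor layouts after resetting a fake elevator, rotate the tower room and shift time.
; Case events reveal and register interactive boxes, some polling the split state before firing console-command events.
; SetRelatedObjects links floor boxes to their LightHouseS and CubeHouseS counterparts from the game instance.
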(event Custom|ThirdCaseStart
  (bind _mesh_wine_box_cap (Variables|Default|GetMesh_Wine_Box_Cap))
  (bind _3rdcasebox (Variables|Default|Get3rdCaseBox))
  (Transformation|AttachComponentToComponent _mesh_wine_box_cap (Variables|Default|Get3rdCaseBox) "None" "KeepWorld" "KeepWorld" "KeepWorld" false)
  (Transformation|SetRelativeLocation _mesh_wine_box_cap (Math|Vector|MakeVector 0.0 0.0 -76.0) false false)
  (Transformation|SetRelativeRotation _mesh_wine_box_cap (Math|Rotator|MakeRotator 0.0 0.0 1.8e+02) false false)
  (for _array_element (Components|GetChildrenComponents _3rdcasebox false)
    (Development|SetHiddeninGame _array_element false true)
    (bind _asbp_interactive_basic (Utilities|Casting|CastToBP_Interactive_Basic (Variables|/Script/Engine.ChildActorComponent|GetChildActor _3rdcasebox)))
    (Default|SetRelatedCollision _asbp_interactive_basic "QueryOnly")
    (Utilities|Array|Add (Variables|Default|GetInteractiveBoxes) _3rdcasebox)))

(event Custom|HideWalls
  ;[1 1 1] HideWalls
  (bind _isa (Utilities|FlowControl|FlipFlop)
    (:A
      (bind _fade (Timeline|WallsFade Play)
        (:Update
          (Rendering|Material|SetScalarParameterValue (Variables|WallDynamicMaterial|GetDynamicBrickMat) "FadeAmount" _fade :!class /Script/Engine.MaterialInstanceDynamic)
          (Rendering|Material|SetScalarParameterValue (Variables|WallDynamicMaterial|GetDynamicConcreteMat) "FadeAmount" _fade :!class /Script/Engine.MaterialInstanceDynamic)
          (Rendering|Material|SetScalarParameterValue (Variables|WallDynamicMaterial|GetDynamicWoodMat) "FadeAmount" _fade :!class /Script/Engine.MaterialInstanceDynamic)
          (Rendering|Material|SetScalarParameterValue (Variables|WallDynamicMaterial|GetDynamicRoofMat) "FadeAmount" _fade :!class /Script/Engine.MaterialInstanceDynamic)
          (Rendering|Material|SetScalarParameterValue (Variables|WallDynamicMaterial|GetDynamicRoofMat2) "FadeAmount" _fade :!class /Script/Engine.MaterialInstanceDynamic)
          (Rendering|Material|SetScalarParameterValue (Variables|WallDynamicMaterial|GetDynamicBrickMat2) "FadeAmount" _fade :!class /Script/Engine.MaterialInstanceDynamic))
        (:Finished
          (Variables|Default|SetisWallsHide _isa))))
    (:B
      (Timeline|WallsFade Reverse))))

(event Custom|FirstCaseStart
  (bind _1stcasebox (Variables|Default|Get1stCaseBox))
  (for _array_element (Components|GetChildrenComponents _1stcasebox false)
    (Development|SetHiddeninGame _array_element false true)
    (bind _asbp_interactive_basic (Utilities|Casting|CastToBP_Interactive_Basic (Variables|/Script/Engine.ChildActorComponent|GetChildActor _1stcasebox)))
    (Default|SetRelatedCollision _asbp_interactive_basic "QueryOnly")
    (Utilities|Array|Add (Variables|Default|GetInteractiveBoxes) _1stcasebox)))

(event Custom|FinalTrick
  (bind _sphere (Variables|Default|GetSphere))
  (bind _headbox (Variables|Default|GetHeadBox))
  (Transformation|AttachComponentToComponent _sphere (Variables|FloorComps|Get时之灯塔_TowerPlat) "None" "KeepWorld" "KeepWorld" "KeepWorld" false)
  (Transformation|SetRelativeLocation _sphere "230.000000,20.000000,1100.000000" false false)
  (Transformation|SetRelativeRotation _sphere "0, 0, 0" false false)
  (Development|SetHiddeninGame (Variables|Default|GetStaticMesh1) false false)
  (Physics|SetSimulatePhysics _sphere true)
  (bind _asbp_interactive_basic (Utilities|Casting|CastToBP_Interactive_Basic (Variables|/Script/Engine.ChildActorComponent|GetChildActor _headbox)))
  (Default|SetRelatedCollision _asbp_interactive_basic "QueryOnly")
  (Utilities|Array|Add (Variables|Default|GetInteractiveBoxes) _headbox))

(event Custom|SecondCaseStart
  (bind _2ndcasebox (Variables|Default|Get2ndCaseBox))
  (for _array_element (Components|GetChildrenComponents _2ndcasebox false)
    (Development|SetHiddeninGame _array_element false true)
    (bind _asbp_interactive_basic (Utilities|Casting|CastToBP_Interactive_Basic (Variables|/Script/Engine.ChildActorComponent|GetChildActor _2ndcasebox)))
    (Default|SetRelatedCollision _asbp_interactive_basic "QueryOnly")
    (Utilities|Array|Add (Variables|Default|GetInteractiveBoxes) _2ndcasebox)
    (if (== (Variables|Default|GetSplitState) 1) :!label _label
      (Utilities|FlowControl|Delay 2.6)
      (Default|SetCameraRotation (Variables|Reference|GetRoomControllerRef) "-40.000000,40.000000,0.000000")
      (Development|ExecuteConsoleCommand "ce SplitFloors" 0)
      (Development|ExecuteConsoleCommand "ce HideWalls" 0)
      (else
        (Utilities|FlowControl|Delay 0.5)
        (goto _label)))))

(event Custom|FinalTrickPre
  (Physics|SetSimulatePhysics (Variables|Default|GetSphere) false)
  (if (== (Variables|Default|GetSplitState) 1) :!label _label
    (Utilities|FlowControl|Delay 2.6)
    (Development|ExecuteConsoleCommand "ce SplitFloors" 0)
    (Utilities|FlowControl|Delay 1.6)
    (Default|CallFinalTrickRecall)
    (else
      (Utilities|FlowControl|Delay 0.5)
      (goto _label))))

(event EventTowerRoomMove
  (params (TowerRoomState :type Integer))
  (bind _returnvalue (* TowerRoomState 90))
  (bind _towerroomrotatecontainer (Variables|Default|GetTowerRoomRotateContainer))
  (bind _returnvalue_2 (Math|Conversions|ToFloat(Integer) _returnvalue))
  ;[1 1 1] RotateRoom
  (Variables|Private|SetRoomRotationTemp (.yaw (Variables|/Script/Engine.SceneComponent|GetRelativeRotation _towerroomrotatecontainer)))
  (bind _angle (Timeline|RoomRotate PlayFromStart)
    (:Update
      (Transformation|SetRelativeRotation _towerroomrotatecontainer (Math|Rotator|MakeRotator 0.0 0.0 (Utilities|CalcDeltaDist (Math|Float|SelectFloat (+ _returnvalue_2 3.6e+02) _returnvalue_2 (> (Variables|Private|GetRoomRotationTemp) _returnvalue)) (Variables|Private|GetRoomRotationTemp) _angle)) false false))))

(event EventMoveUpFloor
  ;[1 1 1] Elevator(Fake)
  (if (and (> (Variables|State|GetElevatorState) 0) (not (Variables|状态|GetisElevatorMoving)))
    (Variables|状态|SetisElevatorMoving true)
    (Math|Integer|DecrementInt (Variables|State|GetElevatorState)
      (:%20%20
        (Utilities|FlowControl|Delay 1.0)
        (Variables|状态|SetisElevatorMoving false)))))

(event EventMoveDownFloor
  ;[1 1 1] Elevator(Fake)
  (if (and (< (Variables|State|GetElevatorState) 2) (not (Variables|状态|GetisElevatorMoving)))
    (Variables|状态|SetisElevatorMoving true)
    (Math|Integer|IncrementInt (Variables|State|GetElevatorState)
      (:%20%20
        (Utilities|FlowControl|Delay 1.0)
        (Variables|状态|SetisElevatorMoving false)))))

(event EventChangeTimeSp
  (bind _defaultsceneroot (Variables|组件|GetDefaultSceneRoot))
  (bind _towerroomscalecontainer (Variables|Default|GetTowerRoomScaleContainer))
  (bind _returnvalue (Transformation|GetWorldLocation _defaultsceneroot))
  ;[1 1 1] ChangeTime
  (if (Variables|/Game/WorldInferRules/GI_Room_Instance.GI_Room_Instance_C|GetisCubeHouseSp (Variables|Reference|GetRoomInstanceRef))
    (Transformation|SetRelativeScale3D _towerroomscalecontainer "1.000000,-1.000000,1.000000")
    (Transformation|SetRelativeRotation _towerroomscalecontainer "0.000000,-90.000000,0.000000" false false))
  (Development|SetHiddeninGame (Variables|Default|Get时之灯塔_TowerRoomS) true true)
  (bind _move (Timeline|TimeChange Play)
    (:Update
      (Transformation|SetWorldLocation _defaultsceneroot (Math|Vector|MakeVector (.x _returnvalue) _move (.z _returnvalue)) false false))))

(event EventSplitFloors
  ;[1 1 1] SplitFloors
  (if (not (Variables|状态|GetisElevatorMoving))
    (Utilities|WhileLoopwithDelay (> (Variables|State|GetElevatorState) 0) 1.0
      (:LoopBody
        (CallFunction|MoveUpFloor))
      (:Completed
        (Utilities|FlowControl|MultiGate false true -1
          (:Out%200
            (Variables|Default|SetSplitState 0)
            (bind (_direction _roof _floor3 _floor2) (Timeline|FloorSplit1 Play)
              (:Update
                (Utilities|SplitFloorbyDistance (Math|Vector|MakeVector (- 0.0 (stale _x)) (- 0.0 (stale _y)) (- _roof (stale _z))) (Math|Vector|MakeVector (stale _x) (- 0.0 (stale _y)) _floor3) (Math|Vector|MakeVector (- 0.0 (stale _x)) (stale _y) (+ _floor2 (stale _z))) (Math|Vector|MakeVector (stale _x) (stale _y) (+ (stale _z) (stale _z))) :!label _label))))
          (:Out%201
            (Variables|Default|SetSplitState 1)
            (bind (_direction_2 _x _y _z) (Timeline|FloorSplit2 Play)
              (:Update
                (goto _label))))
          (:Out%202
            (Variables|Default|SetSplitState 2)
            (Utilities|FlowControl|Sequence
              (:then_0
                (Timeline|FloorSplit1 Reverse))
              (:then_1
                (Timeline|FloorSplit2 Reverse)))))))))

(event EventChangeTimeNormal
  (bind _defaultsceneroot (Variables|组件|GetDefaultSceneRoot))
  (bind _towerroomscalecontainer (Variables|Default|GetTowerRoomScaleContainer))
  (bind _returnvalue (Transformation|GetWorldLocation _defaultsceneroot))
  ;[1 1 1] ChangeTime
  (Transformation|SetRelativeScale3D _towerroomscalecontainer "1.000000,1.000000,1.000000")
  (Transformation|SetRelativeRotation _towerroomscalecontainer "0, 0, 0" false false)
  (Development|SetHiddeninGame (Variables|Default|Get时之灯塔_TowerRoomS) false true)
  (bind _move (Timeline|TimeChange Reverse)
    (:Update
      (Transformation|SetWorldLocation _defaultsceneroot (Math|Vector|MakeVector (.x _returnvalue) _move (.z _returnvalue)) false false))))

(event EventBeginPlay
  (Utilities|FlowControl|Sequence
    (:then_0
      (bind _aspc_room_controller (Utilities|Casting|CastToPC_RoomController (Game|GetPlayerController 0)))
      (Variables|Reference|SetRoomControllerRef _aspc_room_controller)
      (bind _asgi_room_instance (Utilities|Casting|CastToGI_Room_Instance (Game|GetGameInstance)))
      (Variables|Reference|SetRoomInstanceRef _asgi_room_instance))
    (:then_1
      (Utilities|DamagedMaterialSolve))))

(fn ConstructionScript
  (Utilities|FlowControl|Sequence
    (:then_0
      (Variables|Default|SetInteractiveBoxes (Utilities|Array|MakeArray (Variables|BoxComps|GetFloor1Box) (Variables|Default|GetTowerFloorBox) (Variables|BoxComps|GetFloor2Box) (Variables|BoxComps|GetFloor3Box) (Variables|BoxComps|GetFloor4Box) (Variables|Default|GetTowerPlatBox) (Variables|Default|GetTowerRoomBox))))
    (:then_1
      (Utilities|HideCaseObjectCollision))))

(fn SetRelatedObjects
  (bind _asgi_room_instance (Utilities|Casting|CastToGI_Room_Instance (Game|GetGameInstance)))
  (Utilities|FlowControl|Sequence
    (:then_0
      ;[1 1 1] SetRelatedObject
      (bind _asbp_interactive_basic (Utilities|Casting|CastToBP_Interactive_Basic (Variables|/Script/Engine.ChildActorComponent|GetChildActor (Variables|/Game/WorldInferRules/BP_Room_LightHouse_S.BP_Room_LightHouse_S_C|GetFloor1Box (Variables|/Game/WorldInferRules/GI_Room_Instance.GI_Room_Instance_C|GetlightHouseS _asgi_room_instance)))))
      (bind _asbp_interactive_basic_2 (Utilities|Casting|CastToBP_Interactive_Basic (Variables|/Script/Engine.ChildActorComponent|GetChildActor (Variables|/Game/WorldInferRules/BP_Room_CubeHouse_S.BP_Room_CubeHouse_S_C|GetFloor1Box (Variables|/Game/WorldInferRules/GI_Room_Instance.GI_Room_Instance_C|GetcubeHouseS _asgi_room_instance)))))
      (bind _asbp_interactive_basic_3 (Utilities|Casting|CastToBP_Interactive_Basic (Variables|/Script/Engine.ChildActorComponent|GetChildActor (Variables|BoxComps|GetFloor1Box))))
      (Variables|/Game/WorldInferRules/BP_Interactive_Basic.BP_Interactive_Basic_C|SetrelatedInteractive _asbp_interactive_basic_3 (Utilities|Array|MakeArray _asbp_interactive_basic))
      (Variables|/Game/WorldInferRules/BP_Interactive_Basic.BP_Interactive_Basic_C|SetrelatedInteractiveSp _asbp_interactive_basic_3 (Utilities|Array|MakeArray _asbp_interactive_basic_2)))
    (:then_1
      (bind _asbp_interactive_basic_4 (Utilities|Casting|CastToBP_Interactive_Basic (Variables|/Script/Engine.ChildActorComponent|GetChildActor (Variables|/Game/WorldInferRules/BP_Room_LightHouse_S.BP_Room_LightHouse_S_C|GetFloor2Box (Variables|/Game/WorldInferRules/GI_Room_Instance.GI_Room_Instance_C|GetlightHouseS _asgi_room_instance)))))
      (bind _asbp_interactive_basic_5 (Utilities|Casting|CastToBP_Interactive_Basic (Variables|/Script/Engine.ChildActorComponent|GetChildActor (Variables|/Game/WorldInferRules/BP_Room_CubeHouse_S.BP_Room_CubeHouse_S_C|GetFloor2Box (Variables|/Game/WorldInferRules/GI_Room_Instance.GI_Room_Instance_C|GetcubeHouseS _asgi_room_instance)))))
      (bind _asbp_interactive_basic_6 (Utilities|Casting|CastToBP_Interactive_Basic (Variables|/Script/Engine.ChildActorComponent|GetChildActor (Variables|BoxComps|GetFloor2Box))))
      (Variables|/Game/WorldInferRules/BP_Interactive_Basic.BP_Interactive_Basic_C|SetrelatedInteractive _asbp_interactive_basic_6 (Utilities|Array|MakeArray _asbp_interactive_basic_4))
      (Variables|/Game/WorldInferRules/BP_Interactive_Basic.BP_Interactive_Basic_C|SetrelatedInteractiveSp _asbp_interactive_basic_6 (Utilities|Array|MakeArray _asbp_interactive_basic_5)))
    (:then_2
      (bind _asbp_interactive_basic_7 (Utilities|Casting|CastToBP_Interactive_Basic (Variables|/Script/Engine.ChildActorComponent|GetChildActor (Variables|/Game/WorldInferRules/BP_Room_LightHouse_S.BP_Room_LightHouse_S_C|GetFloor3Box (Variables|/Game/WorldInferRules/GI_Room_Instance.GI_Room_Instance_C|GetlightHouseS _asgi_room_instance)))))
      (bind _asbp_interactive_basic_8 (Utilities|Casting|CastToBP_Interactive_Basic (Variables|/Script/Engine.ChildActorComponent|GetChildActor (Variables|/Game/WorldInferRules/BP_Room_CubeHouse_S.BP_Room_CubeHouse_S_C|GetFloor3Box (Variables|/Game/WorldInferRules/GI_Room_Instance.GI_Room_Instance_C|GetcubeHouseS _asgi_room_instance)))))
      (bind _asbp_interactive_basic_9 (Utilities|Casting|CastToBP_Interactive_Basic (Variables|/Script/Engine.ChildActorComponent|GetChildActor (Variables|BoxComps|GetFloor3Box))))
      (Variables|/Game/WorldInferRules/BP_Interactive_Basic.BP_Interactive_Basic_C|SetrelatedInteractive _asbp_interactive_basic_9 (Utilities|Array|MakeArray _asbp_interactive_basic_7))
      (Variables|/Game/WorldInferRules/BP_Interactive_Basic.BP_Interactive_Basic_C|SetrelatedInteractiveSp _asbp_interactive_basic_9 (Utilities|Array|MakeArray _asbp_interactive_basic_8)))
    (:then_3
      (bind _asbp_interactive_basic_10 (Utilities|Casting|CastToBP_Interactive_Basic (Variables|/Script/Engine.ChildActorComponent|GetChildActor (Variables|/Game/WorldInferRules/BP_Room_LightHouse_S.BP_Room_LightHouse_S_C|GetFloor4Box (Variables|/Game/WorldInferRules/GI_Room_Instance.GI_Room_Instance_C|GetlightHouseS _asgi_room_instance)))))
      (bind _asbp_interactive_basic_11 (Utilities|Casting|CastToBP_Interactive_Basic (Variables|/Script/Engine.ChildActorComponent|GetChildActor (Variables|/Game/WorldInferRules/BP_Room_CubeHouse_S.BP_Room_CubeHouse_S_C|GetFloor4Box (Variables|/Game/WorldInferRules/GI_Room_Instance.GI_Room_Instance_C|GetcubeHouseS _asgi_room_instance)))))
      (bind _asbp_interactive_basic_12 (Utilities|Casting|CastToBP_Interactive_Basic (Variables|/Script/Engine.ChildActorComponent|GetChildActor (Variables|BoxComps|GetFloor4Box))))
      (Variables|/Game/WorldInferRules/BP_Interactive_Basic.BP_Interactive_Basic_C|SetrelatedInteractive _asbp_interactive_basic_12 (Utilities|Array|MakeArray _asbp_interactive_basic_10))
      (Variables|/Game/WorldInferRules/BP_Interactive_Basic.BP_Interactive_Basic_C|SetrelatedInteractiveSp _asbp_interactive_basic_12 (Utilities|Array|MakeArray _asbp_interactive_basic_11)))))